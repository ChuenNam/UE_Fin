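; BP_Door is a proximity door that swings open when BP_MyPlayer enters its Box trigger and closes when the player leaves.
; The overlap events set CanOpen and call OpenDoor, which plays or reverses a single timeline accordingly.
; The timeline track drives the Door component's relative yaw on each update, alongside a leftover-looking debug print.
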(event `OpenDoor`
  (if (`self.CanOpen`)
    (bind (_direction `_新建轨道_0`) (`Timeline|时间轴` :!label _label)
      (:`Update`
        (`SceneComponent.K2_SetRelativeRotation` (`self.Door`) (`KismetMathLibrary.MakeRotator` 0.0 0.0 `_新建轨道_0`) false false)
        (`KismetSystemLibrary.PrintString` "6")))
    (else
      (goto _label :!via `Reverse`))))

(event `self.Box.OnComponentBeginOverlap`
  (params (OverlappedComponent :type "PrimitiveComponent Object Reference") (OtherActor :type "Actor Object Reference") (OtherComp :type "PrimitiveComponent Object Reference") (OtherBodyIndex :type Integer) (bFromSweep :type Boolean) (SweepResult :type "HitResult Structure (by ref)"))
  (bind _asbp_my_player (cast `/Game/BP/BP_MyPlayer` OtherActor))
  (`/Engine/EditorBlueprintResources/StandardMacros.IsValid` _asbp_my_player
    (:`Is Valid`
      (set `self.CanOpen` true)
      (`self.OpenDoor`))))

(event `self.Box.OnComponentEndOverlap`
  (params (OverlappedComponent :type "PrimitiveComponent Object Reference") (OtherActor :type "Actor Object Reference") (OtherComp :type "PrimitiveComponent Object Reference") (OtherBodyIndex :type Integer))
  (bind _asbp_my_player (cast `/Game/BP/BP_MyPlayer` OtherActor))
  (`/Engine/EditorBlueprintResources/StandardMacros.IsValid` _asbp_my_player
    (:`Is Valid`
      (set `self.CanOpen` false)
      (`self.OpenDoor`))))

(fn `UserConstructionScript`)